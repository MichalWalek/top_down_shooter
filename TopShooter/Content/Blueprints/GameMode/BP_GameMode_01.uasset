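; Game mode that drives enemy waves by spawning spiders at random points in the level.
; Two seconds after BeginPlay, NewWave increments CurrentWave and starts a looping timer that calls SpawnWave every couple of seconds.
; Each tick spawns one BP_Spider_01 at a randomly chosen TargetPoint, gathered from all such actors in the level.
; The timer is never cleared here, so spawning continues indefinitely within the first wave.
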(event Custom|SpawnWave
  (CallFunction|SpawnSpider))

(event EventBeginPlay
  (Utilities|FlowControl|Delay 2.0)
  (CallFunction|NewWave))

(fn ConstructionScript)

(fn NewWave
  (Math|Integer|IncrementInt (Variables|Default|GetCurrentWave)
    (:%20%20
      (bind _returnvalue (Utilities|Time|SetTimerbyFunctionName 0 "SpawnWave" 2.0 true))
      (return _returnvalue))))

(fn RandomSpawnPoint
  (bind _outactors (Actor|GetAllActorsOfClass "/Script/Engine.TargetPoint"))
  (return (Utilities|Array|Get(acopy) _outactors (Math|Random|RandomIntegerinRange 0 (Utilities|Array|LastIndex _outactors)))))

(fn SpawnSpider
  (bind _output (CallFunction|RandomSpawnPoint))
  (Utilities|IsValid _output
    (:Is%20Valid
      (Game|SpawnActorfromClass "/Game/Blueprints/Pawns/BP_Spider_01.BP_Spider_01_C" (Transformation|GetActorTransform _output) "Undefined" 0 0))))