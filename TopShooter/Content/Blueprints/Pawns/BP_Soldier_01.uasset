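; BP_Soldier_01 is a player-controlled soldier pawn that moves along fixed world X and Y axes from forward/back and left/right input.
; Each tick it derives mouse velocity from the frame's mouse delta and delta seconds.
; When that speed exceeds a dead-zone threshold, it interpolates the controller's yaw toward the direction of mouse motion, computed with atan2.
; Despite its name, IsMouseDeadZone returns true outside the dead zone.
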(event EventTick
  (params (DeltaSeconds :type Float%20%28single-precision%29))
  (CallFunction|UpdataPlayerRotation))

(event Input|AxisEvents|InputAxisMoveForwardBack
  (params (AxisValue :type Float%20%28single-precision%29))
  (Pawn|Input|AddMovementInput "1.000000, 0, 0" AxisValue false))

(event Input|AxisEvents|InputAxisMoveLeftRight
  (params (AxisValue :type Float%20%28single-precision%29))
  (Pawn|Input|AddMovementInput "0,1.000000, 0" AxisValue false))

(fn ConstructionScript)

(fn GetMouseVelocity
  (bind _returnvalue (Game|GetPlayerController 0))
  (bind (_deltax _deltay) (Class|PlayerController|GetInputMouseDelta _returnvalue))
  (return (/ (Math|Vector2D|MakeVector2D _deltax _deltay) (Utilities|Time|GetWorldDeltaSeconds))))

(fn UpdataPlayerRotation
  (bind _returnvalue (Game|GetPlayerController 0))
  (bind _returnvalue_2 (CallFunction|GetMouseVelocity))
  (if (CallFunction|IsMouseDeadZone)
    (Pawn|SetControlRotation _returnvalue (Math|Interpolation|RInterpTo (Pawn|GetControlRotation _returnvalue :!class /Script/Engine.Controller) (Math|Rotator|MakeRotator 0.0 0.0 (Class|KismetMathLibrary|DegAtan2 (.x _returnvalue_2) (.y _returnvalue_2))) (Utilities|Time|GetWorldDeltaSeconds) (Variables|Default|GetDeltaTimeMultiply)))))

(fn IsMouseDeadZone
  (return (> (Math|Vector2D|Vector2DLength (CallFunction|GetMouseVelocity)) (Variables|Default|GetMouseDeadZone))))